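; Player character Blueprint that toggles the pause menu from the IA_Pause Enhanced Input action.
; The first press creates and shows WBP_PauseMenu, switches to Game and UI input with a visible cursor, and pauses the game.
; The next press removes the widget, unpauses, and restores game-only input with a hidden cursor, tracking state with IsPauseMenuOpen.
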(event `EnhancedInput|/Game/Input/InputActions/IA_Pause`
  (params (ActionValue :type Boolean) (ElapsedSeconds :type "Float (double-precision)") (TriggeredSeconds :type "Float (double-precision)") (InputAction :type "InputAction Object Reference" :default "/Game/Input/InputActions/IA_Pause.IA_Pause"))
  (bind _returnvalue (`GameplayStatics.GetPlayerController` 0))
  (bind _returnvalue_2 (`GameplayStatics.GetPlayerController` 0))
  (:`Started`
    (if (not (`self.IsPauseMenuOpen`))
      (set `self.IsPauseMenuOpen` true)
      (bind _returnvalue_3 (`|GenericCreateObject` _returnvalue_2 "/Game/Blueprints/UI/WBP_PauseMenu.WBP_PauseMenu_C"))
      (bind _output_get (set `self.Pause Menu` _returnvalue_3))
      (`UserWidget.AddToViewport` _output_get 0)
      (`WidgetBlueprintLibrary.SetInputMode_GameAndUIEx` _returnvalue_2 null)
      (set `PlayerController.bShowMouseCursor` true _returnvalue_2)
      (`GameplayStatics.SetGamePaused` true)
      (else
        (set `self.IsPauseMenuOpen` false)
        (`Widget.RemoveFromParent` (`self.Pause Menu`))
        (`GameplayStatics.SetGamePaused` false)
        (`WidgetBlueprintLibrary.SetInputMode_GameOnly` _returnvalue)
        (set `PlayerController.bShowMouseCursor` false _returnvalue)))))

(fn `UserConstructionScript`)